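; Inventory item actor that the top-down character picks up by overlapping it.
; On overlap it prints a debug string and passes itself to the character's inventory component.
; Its type is derived rather than stored: Equipment when its EquipmentComponent class is valid, otherwise Consumable.
; Its own PickItem function switches on item type but has no logic in the branches.
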(event EventBeginPlay)

(event Collision|EventActorBeginOverlap
  (params (OtherActor :type Actor%20Object%20Reference))
  (bind _asbp_top_down_character (Utilities|Casting|CastToBP_TopDownCharacter OtherActor))
  (Development|PrintString "Touché")
  (Default|PickItem (Variables|/Game/Exam/Blueprints/BP_TopDownCharacter.BP_TopDownCharacter_C|GetBP_InventoryComponent _asbp_top_down_character) self))

(fn ConstructionScript)

(fn IsEquipment
  (return (Utilities|IsValidClass (Variables|Default|GetEquipmentComponent))))

(fn GetItemType
  (return (select (CallFunction|IsEquipment) "NewEnumerator1" "NewEnumerator0")))

(fn PickItem
  (params (Item :type BP%20Item%20Object%20Reference))
  (switch Utilities|FlowControl|Switch|SwitchonE_ItemType (CallFunction|GetItemType Item)))